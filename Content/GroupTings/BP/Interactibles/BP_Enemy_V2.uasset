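; BP_Enemy_V2 is a damageable enemy that destroys itself when its health runs out.
; Each GetHurt event subtracts a fixed amount from HealthPoints and spawns an explosion particle effect at the enemy's location.
; Death is detected by polling HealthPoints every Tick rather than checking it when damage is applied.
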(event Custom|GetHurt
  (Variables|CharacterStats|SetHealthPoints (- (Variables|CharacterStats|GetHealthPoints) 1.1))
  (Effects|SpawnEmitteratLocation "/Game/StarterContent/Particles/P_Explosion.P_Explosion" (Transformation|GetActorLocation self)))

(event EventBeginPlay)

(event Collision|EventActorBeginOverlap
  (params (OtherActor :type Actor%20Object%20Reference)))

(event EventTick
  (params (DeltaSeconds :type Float%20%28single-precision%29))
  (if (<= (Variables|CharacterStats|GetHealthPoints) 0.0)
    (Actor|DestroyActor)))

(fn ConstructionScript)