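; BP_EnemyV1 is a draft enemy Blueprint that takes damage through a GetHurt event.
; GetHurt prints a debug message, subtracts a fixed amount from HealthPoints and spawns P_Sparks at the actor's location.
; The death check, which spawns P_Fire and destroys the actor, is disconnected, so the enemy never dies here.
; A BP_HitBox check and a duplicate damage chain are also unwired, and the default events are empty.
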(event Custom|GetHurt
  ;[1 1 1] Draft
  (Development|PrintString "OW!")
  (Variables|CharacterStats|SetHealthPoints (- (Variables|CharacterStats|GetHealthPoints) 1.1))
  (Effects|SpawnEmitteratLocation "/Game/StarterContent/Particles/P_Sparks.P_Sparks" (Transformation|GetActorLocation self)))

(event EventBeginPlay)

(event Collision|EventActorBeginOverlap
  (params (OtherActor :type Actor%20Object%20Reference)))

(event EventTick
  (params (DeltaSeconds :type Float%20%28single-precision%29)))

(fn ConstructionScript)